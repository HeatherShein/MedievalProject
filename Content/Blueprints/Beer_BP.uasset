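; Beer_BP is a pickup actor that a SwordCharacter collects by overlapping it.
; On overlap it spawns a loot pickup particle effect at the character, destroys itself and opens a LootBagWidget.
; The same chain then pauses the game, shows the mouse cursor and sets the character's InventoryItem1 to 1 if it was 0.
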(event `self.ReceiveActorBeginOverlap`
  (params (OtherActor :type "Actor Object Reference"))
  (bind _assword_character (cast `/Game/ThirdPersonBP/Blueprints/SwordCharacter` OtherActor))
  (`GameplayStatics.SpawnEmitterAtLocation` "/Game/InfinityBladeEffects/Effects/FX_Treasure/Loot/P_Loot_Pickup.P_Loot_Pickup" (`self.K2_GetActorLocation` _assword_character))
  (`self.K2_DestroyActor`)
  (bind _returnvalue (`|CreateWidget` "/Game/ThirdPersonBP/Blueprints/LootBagWidget.LootBagWidget_C"))
  (`UserWidget.AddToViewport` _returnvalue 0)
  (`GameplayStatics.SetGamePaused` true)
  (bind _asplayer_controller (cast `PlayerController` (`GameplayStatics.GetPlayerController` 0)))
  (set `PlayerController.bShowMouseCursor` true _asplayer_controller)
  (if (== (`/Game/ThirdPersonBP/Blueprints/SwordCharacter.InventoryItem1` _assword_character) 0)
    (set `/Game/ThirdPersonBP/Blueprints/SwordCharacter.InventoryItem1` 1 _assword_character)))

(fn `UserConstructionScript`)