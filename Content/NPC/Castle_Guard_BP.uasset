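; Castle guard NPC that wanders the navmesh and offers a short dialogue to the player's SwordCharacter.
; A self-repeating AIMoveTo loop walks to random points at a speed randomized on BeginPlay, pausing randomly between moves.
; Box overlap flags the player as in range and prints prompts.
; TalkEvent halts movement and shows two lines in Guard_Dialog_Widget by externally advanced DialogueLine, while leaving restores speed and resets dialogue.
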(event `self.ReceiveBeginPlay`
  ;[1 1 1] Wlak Logic
  (bind _output_get (set `self.WalkSpeed` (`KismetMathLibrary.RandomFloatInRange` 100.0 450.0)))
  (set `CharacterMovementComponent.MaxWalkSpeed` _output_get (`self.CharacterMovement`))
  (`self.WalkEvent`))

(event `WalkEvent`
  ;[1 1 1] Wlak Logic
  (if (not (`self.IsWalking`))
    (`|AIMoveTo` self (`NavigationSystemV1.K2_GetRandomLocationInNavigableRadius` (`self.K2_GetActorLocation`) (`self.WalkRadius`) null null) null
      (:`then`
        (set `self.IsWalking` true))
      (:`OnSuccess`
        (`KismetSystemLibrary.Delay` (`KismetMathLibrary.RandomFloatInRange` 1.0 5.0) :!label _label)
        (set `self.IsWalking` false)
        (`self.WalkEvent`))
      (:`OnFail`
        (goto _label)))))

(event `self.Box.OnComponentBeginOverlap`
  (params (OverlappedComponent :type "PrimitiveComponent Object Reference") (OtherActor :type "Actor Object Reference") (OtherComp :type "PrimitiveComponent Object Reference") (OtherBodyIndex :type Integer) (bFromSweep :type Boolean) (SweepResult :type "HitResult Structure (by ref)"))
  ;[1 1 1] Overlap Logic
  (bind _assword_character (cast `/Game/ThirdPersonBP/Blueprints/SwordCharacter` OtherActor))
  (set `/Game/ThirdPersonBP/Blueprints/SwordCharacter.IsAIOverlapped` true _assword_character)
  (`KismetSystemLibrary.PrintString` "Hello")
  (`KismetSystemLibrary.PrintString` "Print \"E\" to speak"))

(event `self.Box.OnComponentEndOverlap`
  (params (OverlappedComponent :type "PrimitiveComponent Object Reference") (OtherActor :type "Actor Object Reference") (OtherComp :type "PrimitiveComponent Object Reference") (OtherBodyIndex :type Integer))
  ;[1 1 1] Overlap Logic
  (bind _assword_character (cast `/Game/ThirdPersonBP/Blueprints/SwordCharacter` OtherActor))
  (set `/Game/ThirdPersonBP/Blueprints/SwordCharacter.IsAIOverlapped` false _assword_character)
  (`KismetSystemLibrary.PrintString` "Bye")
  (set `self.IsTalking` false)
  (set `CharacterMovementComponent.MaxWalkSpeed` (`self.WalkSpeed`) (`self.CharacterMovement`))
  (`Widget.SetVisibility` (stale `TalkEvent` _array_element) "Hidden")
  (set `self.DialogueLine` 0))

(event `TalkEvent`
  (bind _dialogueline (`self.DialogueLine`))
  ;[1 1 1] Dialogue Logic
  (set `CharacterMovementComponent.MaxWalkSpeed` 0.0 (`self.CharacterMovement`))
  (bind _foundwidgets (`WidgetBlueprintLibrary.GetAllWidgetsOfClass` "/Game/NPC/Guard_Dialog_Widget.Guard_Dialog_Widget_C"))
  (for _array_element _foundwidgets
    (if (== _dialogueline 1)
      (set `/Game/NPC/Guard_Dialog_Widget.Dialogue` (`self.Dialogue1`) _array_element)
      (`Widget.SetVisibility` _array_element "Visible")
      (elif (== _dialogueline 2)
        (set `/Game/NPC/Guard_Dialog_Widget.Dialogue` (`self.Dialogue2`) _array_element)
        (`Widget.SetVisibility` _array_element "Visible")
        (elif (>= _dialogueline 3)
          (set `self.DialogueLine` 0)
          (set `/Game/NPC/Guard_Dialog_Widget.Dialogue` "" _array_element))))))

(fn `UserConstructionScript`)